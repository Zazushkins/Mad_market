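; BP_Spawner_Oculus9 is a looping spawner that periodically places a randomly chosen actor through its ChildActor component.
; After a long initial delay it sets the child actor class to a random entry from the Random array, waits longer, then calls SpawnerOcul to restart the cycle.
; Each cycle replaces the previous child actor, and a sound playback node is left unconnected.
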(event `self.ReceiveBeginPlay`
  (bind _random (`self.random`))
  ;[1 1 1] Spawn obj
  (`KismetSystemLibrary.Delay` 160.0 :!label _label)
  (`ChildActorComponent.SetChildActorClass` (`self.ChildActor`) (`|GetArrayItem` _random (`KismetMathLibrary.RandomIntegerInRange` 0 (- (`KismetArrayLibrary.Array_Length` _random) 1))))
  (`KismetSystemLibrary.Delay` 380.0)
  (`self.spawnerOcul`))

(event `spawnerOcul`
  ;[1 1 1] Spawn obj
  (goto _label))

(fn `UserConstructionScript`)