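; Spawner Blueprint that periodically sets its ChildActor component to a class picked from the Random array.
; BeginPlay starts a delayed cycle: wait, set the class, wait longer, then repeat through the SpawnOcul event.
; The random index range runs from zero to the negated array length, so it does not span the array's valid indices.
; A thunder-and-rain sound node is left unconnected and never plays.
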(event `self.ReceiveBeginPlay`
  (bind _random (`self.Random`))
  ;[1 1 1] Spawn obj
  (`KismetSystemLibrary.Delay` 100.0 :!label _label)
  (`ChildActorComponent.SetChildActorClass` (`self.ChildActor`) (`|GetArrayItem` _random (`KismetMathLibrary.RandomIntegerInRange` 0 (- 0 (`KismetArrayLibrary.Array_Length` _random)))))
  (`KismetSystemLibrary.Delay` 320.0)
  (`self.SpawnOcul`))

(event `SpawnOcul`
  ;[1 1 1] Spawn obj
  (goto _label))

(fn `UserConstructionScript`)