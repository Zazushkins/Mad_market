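; BP_Spawn_Oculus is a spawner that keeps swapping its child actor for a random Oculus spawn.
; Five seconds after BeginPlay, it sets the ChildActor component's class to a random entry from the Random array.
; After a further 30-second delay, the SpawnOculus event loops back to the initial delay, repeating the swap indefinitely.
; A PlaySoundAtLocation node is left unconnected and never runs.
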(event `self.ReceiveBeginPlay`
  (bind _random (`self.Random`))
  ;[1 1 1] Spawn obj
  (`KismetSystemLibrary.Delay` 5.0 :!label _label)
  (`ChildActorComponent.SetChildActorClass` (`self.ChildActor`) (`|GetArrayItem` _random (`KismetMathLibrary.RandomIntegerInRange` 0 (- (`KismetArrayLibrary.Array_Length` _random) 1))))
  (`KismetSystemLibrary.Delay` 30.0)
  (`self.SpawnOculus`))

(event `SpawnOculus`
  ;[1 1 1] Spawn obj
  (goto _label))

(fn `UserConstructionScript`)