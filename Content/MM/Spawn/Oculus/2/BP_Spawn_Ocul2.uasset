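; Spawner actor that periodically places a randomly chosen class, apparently an Oculus variant, through its ChildActor component.
; From BeginPlay it waits, sets the child actor class to a random entry of the Random array, then waits longer and calls SpawnOcul to loop back.
; Each cycle replaces the previous child actor.
; A sound-playing node is left disconnected and never runs.
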(event `self.ReceiveBeginPlay`
  (bind _random (`self.Random`))
  ;[1 1 1] Spawn obj
  (`KismetSystemLibrary.Delay` 60.0 :!label _label)
  (`ChildActorComponent.SetChildActorClass` (`self.ChildActor`) (`|GetArrayItem` _random (`KismetMathLibrary.RandomIntegerInRange` 0 (- (`KismetArrayLibrary.Array_Length` _random) 1))))
  (`KismetSystemLibrary.Delay` 280.0)
  (`self.SpawnOcul`))

(event `SpawnOcul`
  ;[1 1 1] Spawn obj
  (goto _label))

(fn `UserConstructionScript`)