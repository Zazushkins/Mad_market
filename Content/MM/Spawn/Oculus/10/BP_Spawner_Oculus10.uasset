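; BP_Spawner_Oculus10 is a spawner that periodically fills its ChildActor component with a random class from the Random array.
; On BeginPlay it checks the level name, running only in Mad_market_Educ or MM_TOVAR, each with its own initial delay.
; Each spawn plays the SuccessfulDelivery sound at world origin and swaps the child actor class.
; After a long wait, SpawnOcul re-enters the level check, repeating the cycle indefinitely.
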(event `self.ReceiveBeginPlay`
  (bind _random (`self.random`))
  (bind _returnvalue (`GameplayStatics.GetCurrentLevelName` true :!label _label))
  (if (`KismetStringLibrary.EqualEqual_StrStr` _returnvalue "Mad_market_Educ")
    (`KismetSystemLibrary.Delay` 20.0)
    ;[1 1 1] Spawn obj
    (`GameplayStatics.PlaySoundAtLocation` "/Game/MM/sound/Successful-Delivery.Successful-Delivery" (0.0 0.0 0.0) (struct) 1.0 1.0 0.0 null null null :!label _label_2)
    (`ChildActorComponent.SetChildActorClass` (`self.ChildActor`) (`|GetArrayItem` _random (`KismetMathLibrary.RandomIntegerInRange` 0 (- (`KismetArrayLibrary.Array_Length` _random) 1))))
    (`KismetSystemLibrary.Delay` 240.0)
    (`self.SpawnOcul`)
    (else
      (bind _returnvalue_2 (`GameplayStatics.GetCurrentLevelName` true))
      (if (`KismetStringLibrary.EqualEqual_StrStr` _returnvalue_2 "MM_TOVAR")
        (`KismetSystemLibrary.Delay` 7.0)
        (goto _label_2)))))

(event `SpawnOcul`
  (goto _label))

(fn `UserConstructionScript`)