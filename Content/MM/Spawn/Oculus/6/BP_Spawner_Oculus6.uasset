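; BP_Spawner_Oculus6 is a timed spawner that repeatedly puts a randomly chosen actor into its ChildActor component.
; From BeginPlay it waits, plays the SuccessfulDelivery sound at the world origin, then sets the child actor class to a random entry from the Random array.
; After a second, longer delay, the SpawnOcul event re-enters the chain at the first delay, so the cycle repeats indefinitely.
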(event `self.ReceiveBeginPlay`
  (bind _random (`self.Random`))
  ;[1 1 1] Spawn obj
  (`KismetSystemLibrary.Delay` 220.0 :!label _label)
  (`GameplayStatics.PlaySoundAtLocation` "/Game/MM/sound/Successful-Delivery.Successful-Delivery" (0.0 0.0 0.0) (struct) 1.0 1.0 0.0 null null null)
  (`ChildActorComponent.SetChildActorClass` (`self.ChildActor`) (`|GetArrayItem` _random (`KismetMathLibrary.RandomIntegerInRange` 0 (- (`KismetArrayLibrary.Array_Length` _random) 1))))
  (`KismetSystemLibrary.Delay` 440.0)
  (`self.SpawnOcul`))

(event `SpawnOcul`
  ;[1 1 1] Spawn obj
  (goto _label))

(fn `UserConstructionScript`)