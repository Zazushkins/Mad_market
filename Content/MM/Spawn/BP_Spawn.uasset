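; BP_Spawn is a spawner that periodically swaps the class of its ChildActor component for a random pick from the Rand array.
; From BeginPlay it waits, plays a storm sound at the world origin, sets the new child class, then waits again.
; The Spawnluj custom event closes the endless loop by re-entering the first delay, giving a swap roughly every 15 seconds.
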(event `self.ReceiveBeginPlay`
  (bind _rand (`self.Rand`))
  ;[1 1 1] Spawn obj
  (`KismetSystemLibrary.Delay` 5.0 :!label _label)
  (`GameplayStatics.PlaySoundAtLocation` "/Game/MM/sound/grozovoy-veter-i-dojd__mp3cut_net_.grozovoy-veter-i-dojd__mp3cut_net_" (0.0 0.0 0.0) (struct) 1.0 1.0 0.0 null null null)
  (`ChildActorComponent.SetChildActorClass` (`self.ChildActor`) (`|GetArrayItem` _rand (`KismetMathLibrary.RandomIntegerInRange` 0 (- (`KismetArrayLibrary.Array_Length` _rand) 1))))
  (`KismetSystemLibrary.Delay` 10.0)
  (`self.Spawnluj`))

(event `Spawnluj`
  ;[1 1 1] Spawn obj
  (goto _label))

(fn `UserConstructionScript`)