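; Puddle spawner that periodically swaps its ChildActor to a random class from the Rand array, active only in the Mad_market_Educ and MM_Luji levels.
; On BeginPlay it checks the level name, waits briefly, plays a storm sound at world origin, then sets the child actor class.
; After a longer delay it calls Spawnluj, which re-enters the level check and repeats the cycle indefinitely.
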(event `self.ReceiveBeginPlay`
  (bind _rand (`self.Rand`))
  ;[1 1 1] Spawn obj
  (bind _returnvalue (`GameplayStatics.GetCurrentLevelName` true :!label _label))
  (if (`KismetStringLibrary.EqualEqual_StrStr` _returnvalue "Mad_market_Educ")
    (`KismetSystemLibrary.Delay` 5.0 :!label _label_2)
    (`GameplayStatics.PlaySoundAtLocation` "/Game/MM/sound/grozovoy-veter-i-dojd__mp3cut_net_.grozovoy-veter-i-dojd__mp3cut_net_" (0.0 0.0 0.0) (struct) 0.15 1.0 0.0 null null null)
    (`ChildActorComponent.SetChildActorClass` (`self.ChildActor`) (`|GetArrayItem` _rand (`KismetMathLibrary.RandomIntegerInRange` 0 (- (`KismetArrayLibrary.Array_Length` _rand) 1))))
    (`KismetSystemLibrary.Delay` 30.0)
    (`self.Spawnluj`)
    (else
      (bind _returnvalue_2 (`GameplayStatics.GetCurrentLevelName` true))
      (if (`KismetStringLibrary.EqualEqual_StrStr` _returnvalue_2 "MM_Luji")
        (goto _label_2)))))

(event `Spawnluj`
  ;[1 1 1] Spawn obj
  (goto _label))

(fn `UserConstructionScript`)